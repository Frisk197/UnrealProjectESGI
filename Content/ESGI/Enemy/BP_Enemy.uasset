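; BP_Enemy is an enemy character that roams at random and chases pawns it sees to attack the player.
; Roam loops between AI moves to random reachable points and random pauses.
; PawnSensing re-arms the attack, raises walk speed and starts a chase; on arrival, HitPlayer sends the enemy's location to BP_MyPlayer's HitEvent.
; A retriggerable delay resumes roaming once sightings stop, without resetting the speed.
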(event OnSeePawn(PawnSensing)
  (params (Pawn :type Pawn%20Object%20Reference))
  (Variables|Default|SetcanAttack true)
  (Utilities|FlowControl|Sequence
    (:then_0
      (Variables|/Script/Engine.CharacterMovementComponent|SetMaxWalkSpeed (Variables|Character|GetCharacterMovement) 5e+02)
      (AI|AIMoveTo self "0, 0, 0" Pawn 1e+01 false
        (:OnSuccess
          (if (Variables|Default|GetcanAttack)
            (Variables|Default|SetcanAttack false)
            (CallFunction|HitPlayer)))))
    (:then_1
      (Utilities|FlowControl|RetriggerableDelay 1e+01)
      (CallFunction|Roam))))

(event Custom|Roam
  (AI|AIMoveTo self (.RandomLocation (AI|Navigation|GetRandomReachablePointinRadius (Transformation|GetWorldLocation (Variables|Character|GetMesh)) 1e+03 0 0)) 0 5.0 false
    (:OnSuccess
      (Utilities|FlowControl|Delay (Math|Random|RandomFloatinRange 0.5 5.0))
      (CallFunction|Roam))))

(event EventBeginPlay
  (CallFunction|Roam))

(fn ConstructionScript)

(fn HitPlayer
  (if (not (Variables|Default|GetplayerHit))
    (Variables|Default|SetplayerHit true)
    (bind _asbp_my_player (Utilities|Casting|CastToBP_MyPlayer (Game|GetPlayerCharacter 0)))
    (Default|HitEvent _asbp_my_player (Transformation|GetActorLocation))
    (Variables|Default|SetplayerHit false)))